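; Paper2D side-scrolling player character with X-axis movement and jumping, a base UI, HP reduced by damage, and a win function that disables movement.
; Each tick derives an Idle, Walk or Jump state from movement and sets the matching flipbook.
; Move input flips the sprite through its X scale.
; Interact checks whether BP_NPC_Guide has the player in range to show or remove its dialogue widget.
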(event Custom|SetUI_NPCGuide
  (bind _returnvalue (UserInterface|CreateWidget "/Game/1144c006_W03/NPC_Guide/Widget/UI_ForNPCGuide.UI_ForNPCGuide_C"))
  (Widget|SetVisibility (Variables|/Game/1144c006_W03/NPC_Guide/Widget/UI_ForNPCGuide.UI_ForNPCGuide_C|GetTxt_NPC_Talk _returnvalue) "Visible")
  (UserInterface|Viewport|AddtoViewport _returnvalue 0))

(event Custom|SET%20UI%20NPCGuide%20Remove
  (Widget|RemovefromParent (stale Custom|SetUI_NPCGuide _returnvalue)))

(event Custom|Set%20UI%20Base
  (bind _returnvalue (UserInterface|CreateWidget "/Game/1144c006_W03/BP_NPC_LookAround/UI_Base.UI_Base_C"))
  (UserInterface|Viewport|AddtoViewport _returnvalue 0))

(event Custom|OnActorBeginOverlap_Event
  (params (OverlappedActor :type Actor%20Object%20Reference) (OtherActor :type Actor%20Object%20Reference)))

(event Input|EnhancedActionEvents|EnhancedInputActionIA_Move01
  (params (ActionValue :type Vector%202D%20Structure) (ElapsedSeconds :type Float%20%28double-precision%29) (TriggeredSeconds :type Float%20%28double-precision%29) (InputAction :type Input%20Action%20Object%20Reference :default "/Game/1144c006_W03/Input/IA_Move01.IA_Move01"))
  (bind _x (Math|Vector2D|BreakVector2D ActionValue))
  (if (Variables|Default|GetCanMove)
    (if (> _x 0.0)
      (Variables|Default|SetIsFacingRight true)
      (else
        (Variables|Default|SetIsFacingRight false)))
    (Pawn|Input|AddMovementInput "1.000000,0.000000,0.000000" _x false)
    (CallFunction|UpdateFacingfromInput (* _x 0.3))
    (else
      (Development|PrintString "Move Locked"))))

(event Input|EnhancedActionEvents|EnhancedInputActionIA_Jump01
  (params (ActionValue :type Boolean) (ElapsedSeconds :type Float%20%28double-precision%29) (TriggeredSeconds :type Float%20%28double-precision%29) (InputAction :type Input%20Action%20Object%20Reference :default "/Game/1144c006_W03/Input/IA_Jump01.IA_Jump01"))
  (:Started
    (Character|Jump))
  (:Completed
    (Character|StopJumping)))

(event Input|EnhancedActionEvents|EnhancedInputActionIA_Interact
  (params (ActionValue :type Boolean) (ElapsedSeconds :type Float%20%28double-precision%29) (TriggeredSeconds :type Float%20%28double-precision%29) (InputAction :type Input%20Action%20Object%20Reference :default "/Game/1144c006_W03/Input/IA_Interact.IA_Interact"))
  (:Started
    (bind _returnvalue (Actor|GetActorOfClass "/Game/1144c006_W03/NPC_Guide/BP_NPC_Guide.BP_NPC_Guide_C"))
    (bind _asbp_npc_guide (Utilities|Casting|CastToBP_NPC_Guide _returnvalue))
    (if (Variables|/Game/1144c006_W03/NPC_Guide/BP_NPC_Guide.BP_NPC_Guide_C|GetPlayerInRange _asbp_npc_guide)
      (CallFunction|SetUINPCGuide)
      (else
        (Development|PrintString "NoNPC")
        (CallFunction|SETUINPCGuideRemove)))))

(event EventBeginPlay
  (Variables|Default|SetRespawn%20Location (Transformation|GetActorLocation))
  (Utilities|FlowControl|Sequence
    (:then_0
      (Input|AddMappingContext (PlayerController|LocalPlayerSubsystems|GetEnhancedInputLocalPlayerSubsystem (Game|GetPlayerController 0)) "/Game/1144c006_W03/Input/IMC_Player.IMC_Player" 0 "(bIgnoreAllPressedKeysUntilRelease=True,bForceImmediately=False,bNotifyUserSettings=False)")
      (CallFunction|SetUIBase)
      ;[0.15 0.15 0.15 0.5] Comment
      (CallFunction|UpdateMoveState)
      (CallFunction|PlayAnimation))
    (:then_1
      (CallFunction|ApplyFacing))))

(event Game|Damage|EventAnyDamage
  (params (Damage :type Float%20%28single-precision%29) (DamageType :type Damage%20Type%20Object%20Reference) (InstigatedBy :type Controller%20Object%20Reference) (DamageCauser :type Actor%20Object%20Reference))
  (Variables|Default|SetHP (- (Variables|Default|GetHP) Damage)))

(event EventTick
  (params (DeltaSeconds :type Float%20%28single-precision%29))
  (CallFunction|UpdateMoveState)
  (CallFunction|PlayAnimation))

(fn ConstructionScript)

(fn UpdateMoveState
  (if (AI|Components|NavMovement|IsFalling (Variables|Character|GetCharacterMovement))
    (Variables|Default|SetAnim_State "NewEnumerator2")
    (elif (> (Math|Float|Absolute(Float) (.X (Math|Vector|BreakVector (Transformation|GetVelocity)))) 5.0)
      (Variables|Default|SetAnim_State "NewEnumerator1")
      (else
        (Variables|Default|SetAnim_State "NewEnumerator0")))))

(fn PlayAnimation
  (bind _paperflipbook (Variables|Default|GetPaperFlipbook))
  (bind _paperflipbook_2 (Variables|Default|GetPaperFlipbook))
  (switch Utilities|FlowControl|Switch|SwitchonEnum_ChangeAnin (Variables|Default|GetAnim_State)
    (:NewEnumerator0
      (Sprite|SetFlipbook _paperflipbook_2 "/Game/U06/Flipbook/FB_Girl_Idle.FB_Girl_Idle"))
    (:NewEnumerator1
      (Sprite|SetFlipbook _paperflipbook_2 "/Game/U06/Flipbook/FB_Girl_Walk.FB_Girl_Walk"))
    (:NewEnumerator2
      (Sprite|SetFlipbook _paperflipbook_2 "/Game/U06/Flipbook/FB_Girl_Jump.FB_Girl_Jump")))
  (Components|Timeline|SetLooping _paperflipbook (Utilities|Enum|NotEqual(Enum) (Variables|Default|GetAnim_State) "NewEnumerator2"))
  (Audio|Components|Audio|Play _paperflipbook))

(fn ApplyFacing
  (Transformation|SetRelativeScale3D (Variables|Default|GetPaperFlipbook) (Math|Vector|MakeVector (Variables|Default|GetFacingSign) 0.3 0.3)))

(fn UpdateFacingfromInput
  (params (AxisValue :type Float%20%28double-precision%29))
  (if (> (Math|Float|Absolute(Float) AxisValue) 0.1)
    (Variables|Default|SetFacingSign (Math|Float|SelectFloat AxisValue -0.3 (> AxisValue 0.0)))
    (CallFunction|ApplyFacing)))

(fn FinalLevel
  (Pawn|Components|CharacterMovement|DisableMovement (Variables|Character|GetCharacterMovement))
  (Variables|Default|SetAnim_State "NewEnumerator0")
  (Development|PrintString "Win"))